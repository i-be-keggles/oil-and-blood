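; BP_Hoverbike is a physics-driven hoverbike that floats above the ground and is steered with Enhanced Input.
; Move input adds forward and sideways force to the static mesh, while Look input adds yaw torque.
; Each tick, a downward trace drives a hover force along the surface normal that fades with height.
; Tick also eases pitch toward the ground slope, zeroes roll and sets damping.
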(event `EnhancedInput|/Game/FirstPerson/Input/Actions/IA_Move`
  (params (ActionValue :type "Vector2D Structure") (ElapsedSeconds :type "Float (double-precision)") (TriggeredSeconds :type "Float (double-precision)") (InputAction :type "InputAction Object Reference" :default "/Game/FirstPerson/Input/Actions/IA_Move.IA_Move"))
  (bind _staticmesh (`self.StaticMesh`))
  (bind _staticmesh_2 (`self.StaticMesh`))
  ;[1 1 1] Strafe
  (:`Triggered`
    (`PrimitiveComponent.AddForce` _staticmesh_2 (* (* ActionValue_Y (`SceneComponent.GetForwardVector` _staticmesh)) (* 30.0 100000.0)) "None" false)
    (`PrimitiveComponent.AddForce` _staticmesh_2 (* (* ActionValue_X (`SceneComponent.GetRightVector` _staticmesh)) (* 20.0 100000.0)) "None" false)))

(event `EnhancedInput|/Game/FirstPerson/Input/Actions/IA_Look`
  (params (ActionValue :type "Vector2D Structure") (ElapsedSeconds :type "Float (double-precision)") (TriggeredSeconds :type "Float (double-precision)") (InputAction :type "InputAction Object Reference" :default "/Game/FirstPerson/Input/Actions/IA_Look.IA_Look"))
  (bind _staticmesh (`self.StaticMesh`))
  (:`Triggered`
    (`PrimitiveComponent.AddTorqueInDegrees` _staticmesh (* (`SceneComponent.GetUpVector` _staticmesh) (* ActionValue_X (* 50.0 1000000000.0))) "None" false)))

(event `self.ReceiveBeginPlay`
  (`|ExecutionSequence`
    (:`then_0`
      ;[1 1 1] Action mapping
      (bind _asplayer_controller (cast `PlayerController` (`self.GetController` (`GameplayStatics.GetPlayerPawn` 0))))
      (bind _returnvalue (pcsubsystem `EnhancedInputLocalPlayerSubsystem` _asplayer_controller))
      (`/Engine/EditorBlueprintResources/StandardMacros.IsValid` _returnvalue
        (:`Is Valid`
          (`EnhancedInputSubsystemInterface.AddMappingContext` _returnvalue "/Game/BigRig/Input/IMC_Vehicle2.IMC_Vehicle2" 0 (struct)))))))

(event `self.ReceiveTick`
  (params (DeltaSeconds :type "Float (single-precision)"))
  (bind _staticmesh (`self.StaticMesh`))
  (bind _staticmesh_2 (`self.StaticMesh`))
  (bind _staticmesh_3 (`self.StaticMesh`))
  (bind _returnvalue (`SceneComponent.K2_GetComponentLocation` _staticmesh_2))
  (bind (_returnvalue_roll _returnvalue_pitch _returnvalue_yaw) (`KismetMathLibrary.BreakRotator` (`SceneComponent.K2_GetComponentRotation` _staticmesh)))
  ;[1 1 1] Hover
  (bind (_outhit _returnvalue_2) (`KismetSystemLibrary.LineTraceSingle` :`Start` _returnvalue :`End` (- _returnvalue (* (`SceneComponent.GetUpVector` _staticmesh_2) (* (`self.GroundHeight`) 1.0))) :`TraceChannel` "TraceTypeQuery1" :`DrawDebugType` "ForDuration"))
  (bind (_returnvalue_roll_2 _returnvalue_pitch_2) (`KismetMathLibrary.BreakRotator` (`KismetMathLibrary.TransformRotation` (`SceneComponent.K2_GetComponentToWorld` _staticmesh) (`KismetMathLibrary.Conv_VectorToRotator` (`KismetMathLibrary.Cross_VectorVector` (`SceneComponent.GetRightVector` (`self.StaticMesh`)) (`.Normal` (`GameplayStatics.BreakHitResult` _outhit)))))))
  (`SceneComponent.K2_SetWorldRotation` (`self.StaticMesh`) (`KismetMathLibrary.MakeRotator` 0.0 (`KismetMathLibrary.Lerp` _returnvalue_pitch (select `bool` _returnvalue_2 :`true` _returnvalue_pitch_2) DeltaSeconds) _returnvalue_yaw) false false)
  (`PrimitiveComponent.AddForce` _staticmesh_3 (* (`.Normal` (`GameplayStatics.BreakHitResult` _outhit)) (`KismetMathLibrary.Lerp` (* (`self.HoverForce`) 1000000.0) 0.0 (/ (`KismetMathLibrary.VSize` (- (`.Location` (`GameplayStatics.BreakHitResult` _outhit)) _returnvalue)) (`self.GroundHeight`)))) "None" false)
  (`PrimitiveComponent.SetLinearDamping` _staticmesh_3 3.0)
  (`PrimitiveComponent.SetAngularDamping` _staticmesh_3 3.0))

(fn `UserConstructionScript`)