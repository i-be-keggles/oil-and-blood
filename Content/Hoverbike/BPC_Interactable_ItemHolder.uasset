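; BPC_Interactable_ItemHolder is an interactable component that acts as a holder for one item carried by the first-person character.
; On Interact, an empty holder takes the player's CarryingItem, clears that reference and snaps the item's mesh to itself, keeping world scale.
; If the player carries nothing, it forwards Interact to the held item's own interactable component and clears HeldItem.
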(event `/Game/Player/BPI_Interactable.Interact`
  (bind _helditem (`self.HeldItem`))
  (bind _asbp_first_person_character (cast `/Game/Player/BP_FirstPersonCharacter` (`GameplayStatics.GetPlayerPawn` 0)))
  (bind _carryingitem (`/Game/Player/BP_FirstPersonCharacter.CarryingItem` _asbp_first_person_character))
  (`/Engine/EditorBlueprintResources/StandardMacros.IsValid` _carryingitem
    (:`Is Valid`
      (`/Engine/EditorBlueprintResources/StandardMacros.IsValid` _helditem
        (:`Is Not Valid`
          (bind _output_get (set `self.HeldItem` _carryingitem))
          (set `/Game/Player/BP_FirstPersonCharacter.CarryingItem` null _asbp_first_person_character)
          (`self.K2_AttachToComponent` (`/Game/Items/Blueprints/BP_Item.Mesh` _output_get) self "None" "SnapToTarget" "SnapToTarget" "KeepWorld" false))))
    (:`Is Not Valid`
      (`/Engine/EditorBlueprintResources/StandardMacros.IsValid` _helditem
        (:`Is Valid`
          (`self.Interact` (`/Game/Items/Blueprints/BP_Item.BPC_Interactable` _helditem))
          (set `self.HeldItem` null))))))