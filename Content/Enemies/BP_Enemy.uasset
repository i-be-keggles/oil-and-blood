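; BP_Enemy is an enemy Blueprint that turns AI perception events into Blackboard data.
; It caches its Blackboard on BeginPlay and handles each perception update by checking the stimulus sense class.
; Sight sets the Target key to the seen actor, or clears it when sight is lost.
; Any other sense writes the stimulus location to TargetLocation, with leftover debug prints labelling it as heard.
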(event `self.ReceiveBeginPlay`
  (set `self.Blackboard` (`AIBlueprintHelperLibrary.GetBlackboard` null)))

(event `self.AIPerception.OnTargetPerceptionUpdated`
  (params (Actor :type "Actor Object Reference") (Stimulus :type "AIStimulus Structure"))
  (bind (_age _expirationage _strength _stimuluslocation _receiverlocation _tag _bsuccessfullysensed) (break `AIStimulus` Stimulus))
  (bind _blackboard (`self.Blackboard`))
  (`KismetSystemLibrary.PrintString` "Hello")
  (bind _returnvalue (`AIPerceptionSystem.GetSenseClassForStimulus` Stimulus))
  (if (== _returnvalue "/Script/AIModule.AISense_Sight")
    (if _bsuccessfullysensed
      (`BlackboardComponent.SetValueAsObject` _blackboard "Target" Actor)
      (else
        (`BlackboardComponent.SetValueAsObject` _blackboard "Target" null)))
    (else
      (`BlackboardComponent.SetValueAsVector` (`self.Blackboard`) "TargetLocation" _stimuluslocation)
      (`KismetSystemLibrary.PrintString` "Heard"))))

(fn `UserConstructionScript`)