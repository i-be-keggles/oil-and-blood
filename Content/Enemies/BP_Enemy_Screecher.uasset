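; BP_Enemy_Screecher is an enemy that raises an alarm when the first-person player character enters its trigger volume.
; On overlap it plays the engage montage and immediately reports a loud, long-range AI noise event at its location with itself as instigator.
; After a short delay it plays the same montage again, and a debug print marks the activation.
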(event `self.Trigger.OnComponentBeginOverlap`
  (params (OverlappedComponent :type "PrimitiveComponent Object Reference") (OtherActor :type "Actor Object Reference") (OtherComp :type "PrimitiveComponent Object Reference") (OtherBodyIndex :type Integer) (bFromSweep :type Boolean) (SweepResult :type "HitResult Structure (by ref)"))
  (cast `/Game/Player/BP_FirstPersonCharacter` OtherActor)
  (`|PlayMontage` (`self.SkeletalMesh`) "/Game/Enemies/Screecher/AM_Screecher_Engage.AM_Screecher_Engage"
    (:`then`
      (`KismetSystemLibrary.PrintString` "ScreecherActivated")
      (`AISense_Hearing.ReportNoiseEvent` (`self.K2_GetActorLocation`) 10.0 self 5000.0)
      (`KismetSystemLibrary.Delay` 1.0)
      (`|PlayMontage` (`self.SkeletalMesh`) "/Game/Enemies/Screecher/AM_Screecher_Engage.AM_Screecher_Engage"))))

(fn `UserConstructionScript`
  (`parent.UserConstructionScript`))