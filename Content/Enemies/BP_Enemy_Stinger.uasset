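; Stinger enemy Blueprint that uses AI perception and blackboard keys to control when it engages the BigRigSpider rig.
; Perceiving the rig sets it as the Rig key while CanDamageRig is true or a patrol timer is active.
; PatrolRig disables damage and starts a 20-second timer, after which the rig is cleared and damage re-enables following a one-minute cooldown.
; Stingers beginning play within the game's first ten seconds start able to damage it.
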(event `self.ReceiveBeginPlay`
  (`parent.ReceiveBeginPlay`)
  (if (<= (`GameplayStatics.GetTimeSeconds`) 10.0)
    (`BlackboardComponent.SetValueAsBool` (`self.Blackboard`) "CanDamageRig" true)))

(event `self.AIPerception.OnTargetPerceptionUpdated`
  (params (Actor :type "Actor Object Reference") (Stimulus :type "AIStimulus Structure"))
  (bind _asbp_big_rig_spider (cast `/Game/BigRig/BP_BigRigSpider` Actor))
  (if (or (`KismetSystemLibrary.K2_IsValidTimerHandle` (`self.RigPatrolTimer`)) (`BlackboardComponent.GetValueAsBool` (`self.Blackboard`) "CanDamageRig"))
    (`KismetSystemLibrary.PrintString` "Found rig")
    (`BlackboardComponent.SetValueAsObject` (`self.Blackboard`) "Rig" _asbp_big_rig_spider)))

(event `PatrolRig`
  (`BlackboardComponent.SetValueAsBool` (`self.Blackboard`) "CanDamageRig" false)
  (`KismetSystemLibrary.K2_ClearAndInvalidateTimerHandle` (`self.RigPatrolTimer`))
  (bind _returnvalue (`KismetSystemLibrary.K2_SetTimerDelegate` (delegate `StopRigPatroll`) 20.0))
  (set `self.RigPatrolTimer` _returnvalue))

(event `StopRigPatroll`
  (`KismetSystemLibrary.K2_ClearAndInvalidateTimerHandle` (`self.RigPatrolTimer`))
  (`BlackboardComponent.SetValueAsObject` (`self.Blackboard`) "Rig" null)
  (`KismetSystemLibrary.Delay` 60.0)
  (`BlackboardComponent.SetValueAsBool` (`self.Blackboard`) "CanDamageRig" true)
  (`KismetSystemLibrary.PrintString` "Abandoning rig"))

(fn `UserConstructionScript`
  (`parent.UserConstructionScript`))