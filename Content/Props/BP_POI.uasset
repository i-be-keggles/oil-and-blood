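; Point of interest actor that procedurally scatters structures, props and items around itself on BeginPlay.
; Each category gets a random count within its limits, and each spawn is a weighted random pick from that category's list.
; Picks become child actors, or static mesh components as fallback, with random yaw inside a square set by Radius.
; A final pass line-traces vertically to snap each root child component to the ground.
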(event `self.ReceiveBeginPlay`
  (bind (_spawnedstructurelimits_x _spawnedstructurelimits_y) (`KismetMathLibrary.BreakVector` (`self.SpawnedStructureLimits`)))
  (bind (_spawnedproplimits_x _spawnedproplimits_y) (`KismetMathLibrary.BreakVector` (`self.SpawnedPropLimits`)))
  (bind (_spawneditemlimits_x _spawneditemlimits_y) (`KismetMathLibrary.BreakVector` (`self.SpawnedItemLimits`)))
  (`self.SpawnWeightedObjects` (`self.Structures`) (`KismetMathLibrary.FTrunc` (`KismetMathLibrary.RandomFloatInRange` _spawnedstructurelimits_x _spawnedstructurelimits_y)))
  (`self.SpawnWeightedObjects` (`self.Props`) (`KismetMathLibrary.FTrunc` (`KismetMathLibrary.RandomFloatInRange` _spawnedproplimits_x _spawnedproplimits_y)))
  (`self.SpawnWeightedObjects` (`self.Items`) (`KismetMathLibrary.FTrunc` (`KismetMathLibrary.RandomFloatInRange` _spawneditemlimits_x _spawneditemlimits_y)))
  (`self.SnapComponentsToGround`))

(event `SpawnWeightedObjects`
  (params (Objects :type "Array of /Game/Props/WeightedObjectSpawn Structure") (Amount :type Integer))
  (bind _radius (`self.Radius`))
  (bind _returnvalue (`KismetMathLibrary.MakeTransform` (`KismetMathLibrary.RandomPointInBoundingBox` (0.0 0.0 0.0) (`KismetMathLibrary.MakeVector` _radius _radius 1.0)) (`KismetMathLibrary.MakeRotator` 0.0 0.0 (`KismetMathLibrary.RandomFloatInRange` 0.0 360.0))))
  (if (> (`KismetArrayLibrary.Array_Length` Objects) 0)
    ;[1 1 1] Set max weight
    (set `self.LocalWeightMax` 0.0)
    (for _array_element Objects
      (set `self.LocalWeightMax` (+ (`self.LocalWeightMax`) (`.Weight_6_C4AF45C8480CEB85AC530F90BA170F26` (break `/Game/Props/WeightedObjectSpawn` _array_element)))))
    ;[1 1 1] Iterate
    (for _ (range 1 (+ Amount 1))
      (set `self.LocalWeight` 0.0)
      (set `self.LocalWeight` (* (`KismetMathLibrary.RandomFloat`) (`self.LocalWeightMax`)))
      ;[1 1 1] Seek random weight
      (for _array_element_2 Objects
        (bind _output_get (set `self.LocalWeight` (- (`self.LocalWeight`) (`.Weight_6_C4AF45C8480CEB85AC530F90BA170F26` (break `/Game/Props/WeightedObjectSpawn` _array_element_2)))))
        ;[1 1 1] Spawn
        (if (<= _output_get 0.0)
          (if (`KismetSystemLibrary.IsValidClass` (break `/Game/Props/WeightedObjectSpawn` _array_element_2))
            (bind _returnvalue_2 (`AddComponent|NODE_AddChildActorComponent-0` :`RelativeTransform` _returnvalue))
            (`ChildActorComponent.SetChildActorClass` _returnvalue_2 (break `/Game/Props/WeightedObjectSpawn` _array_element_2))
            (else
              (`/Engine/EditorBlueprintResources/StandardMacros.IsValid` (`.Mesh_12_7B55ADED490BA9BF7A123699219CD2A8` (break `/Game/Props/WeightedObjectSpawn` _array_element_2))
                (:`Is Valid`
                  (bind _returnvalue_3 (`AddComponent|NODE_AddStaticMeshComponent-0` :`RelativeTransform` _returnvalue))
                  (`StaticMeshComponent.SetStaticMesh` _returnvalue_3 (`.Mesh_12_7B55ADED490BA9BF7A123699219CD2A8` (break `/Game/Props/WeightedObjectSpawn` _array_element_2)))))))
          ;[1 1 1] Break
          (if true
            (break)))))))

(event `SnapComponentsToGround`
  (for _array_element (`SceneComponent.GetChildrenComponents` (`self.DefaultSceneRoot`) false)
    (bind _returnvalue (`SceneComponent.K2_GetComponentLocation` _array_element))
    (bind (_outhit _returnvalue_2) (`KismetSystemLibrary.LineTraceSingle` (+ _returnvalue (0.0 0.0 200.0)) (+ _returnvalue (0.0 0.0 -500.0)) "TraceTypeQuery1"))
    (if _returnvalue_2
      (`SceneComponent.K2_SetWorldLocation` _array_element (`.Location` (`GameplayStatics.BreakHitResult` _outhit)) false true))))

(fn `UserConstructionScript`)