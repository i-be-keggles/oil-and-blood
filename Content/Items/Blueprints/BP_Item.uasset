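; BP_Item is a physics item that the first-person player can pick up, carry and drop.
; BPC_Interactable's OnInteract, when the player carries nothing, registers the item as CarryingItem, disables physics and collision, and snaps the mesh to the player's ItemHolder.
; DropItem teleports the mesh in front of the player's capsule, detaches it, restores physics and collision, and clears CarryingItem.
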(event `self.BPC_Interactable.OnInteract`
  (bind _itemholder (`/Game/Player/BP_FirstPersonCharacter.ItemHolder` (`self.Player`)))
  (bind _asbp_first_person_character (cast `/Game/Player/BP_FirstPersonCharacter` (`Controller.K2_GetPawn` (`GameplayStatics.GetPlayerController` 0))))
  (bind _output_get (set `self.Player` _asbp_first_person_character))
  (`/Engine/EditorBlueprintResources/StandardMacros.IsValid` (`/Game/Player/BP_FirstPersonCharacter.CarryingItem` _asbp_first_person_character)
    (:`Is Not Valid`
      (set `/Game/Player/BP_FirstPersonCharacter.CarryingItem` self _output_get)
      (`PrimitiveComponent.SetSimulatePhysics` (`self.Mesh`) false)
      (`self.SetActorEnableCollision` false)
      (`SceneComponent.K2_AttachToComponent` (`self.Mesh`) _itemholder "None" "KeepWorld" "KeepWorld" "KeepWorld" true)
      (`SceneComponent.K2_SetWorldLocationAndRotation` (`self.Mesh`) (`SceneComponent.K2_GetComponentLocation` _itemholder) (`SceneComponent.K2_GetComponentRotation` _itemholder) false true))))

(event `DropItem`
  (bind _mesh (`self.Mesh`))
  (bind _capsulecomponent (`Character.CapsuleComponent` (`self.Player`)))
  (`SceneComponent.K2_SetWorldLocation` (`self.Mesh`) (+ (`SceneComponent.K2_GetComponentLocation` _capsulecomponent) (* (`SceneComponent.GetForwardVector` _capsulecomponent) 100.0)) false true)
  (`SceneComponent.K2_DetachFromComponent` _mesh "KeepWorld" "KeepWorld" "KeepWorld" true)
  (`PrimitiveComponent.SetSimulatePhysics` _mesh true)
  (`self.SetActorEnableCollision` true)
  (set `/Game/Player/BP_FirstPersonCharacter.CarryingItem` null (`self.Player`)))

(fn `UserConstructionScript`)