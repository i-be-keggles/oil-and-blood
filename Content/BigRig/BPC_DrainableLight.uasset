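; BPC_DrainableLight is a light component on the BigRig spider vehicle, controlled by an interactable switch.
; Initialise stores the switch and its BP_BigRigSpider owner, then binds the switch's interact event to Toggle.
; Toggle records the switch value as active and, only while the rig's battery is on, shows or hides the component and its children to match.
; The SetEnabled event is an empty stub.
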(event `Initialise`
  (params (Switch :type "/Game/BigRig/BPC_Interactable_Switch Object Reference"))
  (bind _output_get (set `self.Switch` Switch))
  (bind _asbp_big_rig_spider (cast `/Game/BigRig/BP_BigRigSpider` (`self.GetOwner` _output_get)))
  (set `self.Rig` _asbp_big_rig_spider)
  (add `/Game/Player/BPC_Interactable.OnInteract` (`self.Switch`) (delegate `Toggle`))
  (`self.Toggle`))

(event `Toggle`
  (bind _output_get (set `self.Active` (`/Game/BigRig/BPC_Interactable_Switch.Value` (`self.Switch`))))
  (if (`/Game/BigRig/BP_BigRigSpider.BatteryOn` (`self.Rig`))
    (`self.SetHiddenInGame` (not _output_get) true)))

(event `SetEnabled`)