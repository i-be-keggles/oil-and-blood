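; Switch interactable component that toggles a boolean state when the player interacts with it.
; Interact flips Value and then fires the OnInteract notification for listeners.
; Observe builds the "[E]" prompt, showing AltPrompt while switched on if one is set and PromptText otherwise.
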(event `/Game/Player/BPI_Interactable.Interact`
  (set `self.Value` (not (`self.Value`)))
  (`self.OnInteract`))

(fn `Observe`
  (returns (Prompt :type String))
  (bind _altprompt (`self.AltPrompt`))
  (return (`KismetStringLibrary.Concat_StrStr` "[E] " (select `bool` (and (not (== _altprompt "")) (`self.Value`)) :`false` (`self.PromptText`) :`true` _altprompt))))