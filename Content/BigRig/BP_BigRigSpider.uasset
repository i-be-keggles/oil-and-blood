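; Drivable spider rig pawn with engine, generator and battery systems operated through interactable switches.
; Looping timers burn fuel (engine by speed through a curve), recharge the battery from the generator, drain it per active light, add wear and update gauge widgets.
; Damage stops the affected system, and an interactable refuels.
; Movement uses FloatingPawnMovement while the engine runs, with a downward trace easing height above ground on move input; a Control Rig maps the skeletal mesh.
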(event `self.ReceiveUnpossessed`
  (params (OldController :type "Controller Object Reference")))

(event `EnhancedInput|/Game/FirstPerson/Input/Actions/IA_Move`
  (params (ActionValue :type "Vector2D Structure") (ElapsedSeconds :type "Float (double-precision)") (TriggeredSeconds :type "Float (double-precision)") (InputAction :type "InputAction Object Reference" :default "/Game/FirstPerson/Input/Actions/IA_Move.IA_Move"))
  (bind _returnvalue (`self.K2_GetActorLocation`))
  ;[1 1 1] Input
  (:`Triggered`
    (if (`self.EngineOn`)
      (`PawnMovementComponent.AddInputVector` (`self.FloatingPawnMovement`) (* (`self.GetActorForwardVector`) ActionValue_Y) false)
      (`self.AddControllerYawInput` (* ActionValue_X 0.1))
      (bind _outhit (`KismetSystemLibrary.LineTraceSingle` (+ _returnvalue (0.0 0.0 1000.0)) (+ _returnvalue (0.0 0.0 -3000.0)) "TraceTypeQuery1"))
      (`self.K2_SetActorLocation` (`KismetMathLibrary.MakeVector` (.x _returnvalue) (.y _returnvalue) (`KismetMathLibrary.Lerp` (.z _returnvalue) (+ (.z (`.Location` (`GameplayStatics.BreakHitResult` _outhit))) (`self.GroundHeight`)) (* 3.0 (`GameplayStatics.GetWorldDeltaSeconds`))))))))

(event `self.ReceiveBeginPlay`
  ;[1 1 1] Start
  (`|ExecutionSequence`
    (:`then_0`
      ;[1 1 1] Setup lights
      (if true
        (`|ExecutionSequence`
          (:`then_0`
            (`/Game/BigRig/BPC_DrainableLight.Initialise` (`self.BPC_DrainableLight_Headlights`) (`self.BPC_Interactable_Switch_Headlights`))
            (`/Game/BigRig/BPC_DrainableLight.Initialise` (`self.BPC_DrainableLight_Rearlights`) (`self.BPC_Interactable_Switch_Rearlight`)))
          (:`then_1`
            (set `self.LightArray` (`|MakeArray` (`self.BPC_DrainableLight_Headlights`) (`self.BPC_DrainableLight_Rearlights`)))))))
    (:`then_1`
      ;[1 1 1] Action mapping
      (bind _asplayer_controller (cast `PlayerController` (`self.GetController` (`GameplayStatics.GetPlayerPawn` 0))))
      (bind _returnvalue (pcsubsystem `EnhancedInputLocalPlayerSubsystem` _asplayer_controller))
      (`/Engine/EditorBlueprintResources/StandardMacros.IsValid` _returnvalue
        (:`Is Valid`
          (`EnhancedInputSubsystemInterface.AddMappingContext` _returnvalue "/Game/BigRig/Input/IMC_Vehicle2.IMC_Vehicle2" 0 (struct)))))
    (:`then_2`
      (`self.StartBattery`))))

(event `StartGenerator`
  ;[1 1 1] Generator
  (if (`/Game/BigRig/BPC_Interactable_ResourceDrain_Damagable.Damaged` (`self.BPC_Interactable_ResourceDrain_Damagable_Generator`))
    (`KismetSystemLibrary.PrintString` "Generator damaged")
    (else
      (bind _output_get (set `self.GeneratorOn` true))
      (set `/Game/BigRig/BPC_Interactable_Switch.Value` _output_get (`self.BPC_Interactable_Switch_Generator`))
      (message `/Game/BigRig/Widgets/BPI_RigWidget.UpdateGeneratorLight` (`WidgetComponent.GetWidget` (`self.EngineLightWidget`)) true)
      (bind _returnvalue (`KismetSystemLibrary.K2_SetTimerDelegate` (delegate `GeneratorDrainFuel`) (`self.EngineUpdateSpeed`) true))
      (set `self.FuelGeneratorDrainTimer` _returnvalue))))

(event `Start Engine`
  ;[1 1 1] Engine
  (if (`/Game/BigRig/BPC_Interactable_ResourceDrain_Damagable.Damaged` (`self.BPC_Interactable_ResourceDrain_Damagable_Engine`))
    (`KismetSystemLibrary.PrintString` "Engine damaged")
    (elif (> (`self.Fuel`) 0.0)
      (bind _output_get (set `self.EngineOn` true))
      (set `/Game/BigRig/BPC_Interactable_Switch.Value` _output_get (`self.BPC_Interactable_Switch_Engine`))
      (message `/Game/BigRig/Widgets/BPI_RigWidget.UpdateEngineLight` (`WidgetComponent.GetWidget` (`self.EngineLightWidget`)) true)
      (bind _returnvalue (`KismetSystemLibrary.K2_SetTimerDelegate` (delegate `EngineDrainFuel`) (`self.EngineUpdateSpeed`) true))
      (set `self.FuelEngineDrainTimer` _returnvalue))))

(event `StopGenerator`
  ;[1 1 1] Generator
  (bind _output_get (set `self.GeneratorOn` false))
  (set `/Game/BigRig/BPC_Interactable_Switch.Value` _output_get (`self.BPC_Interactable_Switch_Generator`))
  (message `/Game/BigRig/Widgets/BPI_RigWidget.UpdateGeneratorLight` (`WidgetComponent.GetWidget` (`self.EngineLightWidget`)) false)
  (`KismetSystemLibrary.K2_ClearAndInvalidateTimerHandle` (`self.FuelGeneratorDrainTimer`)))

(event `Stop Engine`
  ;[1 1 1] Engine
  (bind _output_get (set `self.EngineOn` false))
  (set `/Game/BigRig/BPC_Interactable_Switch.Value` _output_get (`self.BPC_Interactable_Switch_Engine`))
  (`KismetSystemLibrary.K2_ClearAndInvalidateTimerHandle` (`self.FuelEngineDrainTimer`))
  (message `/Game/BigRig/Widgets/BPI_RigWidget.UpdateRPMGauge` (`WidgetComponent.GetWidget` (`self.FuelWidget`)) 0.0)
  (message `/Game/BigRig/Widgets/BPI_RigWidget.UpdateEngineLight` (`WidgetComponent.GetWidget` (`self.EngineLightWidget`)) false))

(event `StartBattery`
  ;[1 1 1] Battery
  (if (`/Game/BigRig/BPC_Interactable_ResourceDrain_Damagable.Damaged` (`self.BPC_Interactable_ResourceDrain_Damagable_Battery`))
    (`KismetSystemLibrary.PrintString` "Battery damaged")
    (else
      (bind _output_get (set `self.BatteryOn` true))
      (set `/Game/BigRig/BPC_Interactable_Switch.Value` _output_get (`self.BPC_Interactable_Switch_Battery`))
      (message `/Game/BigRig/Widgets/BPI_RigWidget.UpdateBatteryLight` (`WidgetComponent.GetWidget` (`self.BatteryWidget`)) true)
      (`self.ReenableLights`)
      (bind _returnvalue (`KismetSystemLibrary.K2_SetTimerDelegate` (delegate `BatteryDrain`) (`self.EngineUpdateSpeed`) true))
      (set `self.BatteryDrainTimer` _returnvalue))))

(event `StopBattery`
  ;[1 1 1] Battery
  (bind _output_get (set `self.BatteryOn` false))
  (set `/Game/BigRig/BPC_Interactable_Switch.Value` _output_get (`self.BPC_Interactable_Switch_Battery`))
  (`self.DisableLights`)
  (message `/Game/BigRig/Widgets/BPI_RigWidget.UpdateBatteryLight` (`WidgetComponent.GetWidget` (`self.BatteryWidget`)) false)
  (`KismetSystemLibrary.K2_ClearAndInvalidateTimerHandle` (`self.BatteryDrainTimer`)))

(event `EngineDrainFuel`
  (bind _returnvalue (`WidgetComponent.GetWidget` (`self.FuelWidget`)))
  (bind _returnvalue_2 (`KismetMathLibrary.FMax` (/ (`KismetMathLibrary.VSize` (`self.GetVelocity`)) (`MovementComponent.GetMaxSpeed` (`self.FloatingPawnMovement`))) (`self.EngineIdleMinPower`)))
  ;[1 1 1] Fuel Drain
  (bind _output_get (set `self.Fuel` (- (`self.Fuel`) (* (* (`self.FuelEngineDrainRate`) (`self.EngineUpdateSpeed`)) (`CurveFloat.GetFloatValue` (`self.FuelCurve`) _returnvalue_2)))))
  (message `/Game/BigRig/Widgets/BPI_RigWidget.UpdateFuelGauge` _returnvalue (/ _output_get (`self.MaxFuel`)))
  (message `/Game/BigRig/Widgets/BPI_RigWidget.UpdateRPMGauge` _returnvalue _returnvalue_2)
  (`/Game/BigRig/BPC_Interactable_ResourceDrain_Damagable.AddWear` (`self.BPC_Interactable_ResourceDrain_Damagable_Engine`) (* _returnvalue_2 (`self.EngineUpdateSpeed`)))
  (if (<= (`self.Fuel`) 0.0)
    (`self.Stop Engine`)
    (`self.StopGenerator`)))

(event `BatteryDrain`
  ;[1 1 1] Battery
  (`|ExecutionSequence`
    (:`then_0`
      (for _array_element (`self.LightArray`)
        (if (`/Game/BigRig/BPC_DrainableLight.Active` _array_element)
          (set `self.BatteryValue` (- (`self.BatteryValue`) (* (`/Game/BigRig/BPC_DrainableLight.DrainRate` _array_element) (`self.EngineUpdateSpeed`)))))))
    (:`then_1`
      (if (<= (`self.BatteryValue`) 0.0)
        (`self.DisableLights`)))
    (:`then_2`
      (message `/Game/BigRig/Widgets/BPI_RigWidget.UpdateBatteryGauge` (`WidgetComponent.GetWidget` (`self.BatteryWidget`)) (/ (`self.BatteryValue`) 100.0))
      (`/Game/BigRig/BPC_Interactable_ResourceDrain_Damagable.AddWear` (`self.BPC_Interactable_ResourceDrain_Damagable_Battery`) (`self.EngineUpdateSpeed`)))))

(event `GeneratorDrainFuel`
  (bind _batteryvalue (`self.BatteryValue`))
  ;[1 1 1] Fuel Drain
  (bind _output_get (set `self.Fuel` (- (`self.Fuel`) (* (`self.FuelGeneratorDrainRate`) (`self.EngineUpdateSpeed`)))))
  (message `/Game/BigRig/Widgets/BPI_RigWidget.UpdateFuelGauge` (`WidgetComponent.GetWidget` (`self.FuelWidget`)) (/ _output_get (`self.MaxFuel`)))
  (if (<= _batteryvalue 0.0)
    (set `self.BatteryValue` 0.0)
    (`self.ReenableLights`))
  (bind _output_get_2 (set `self.BatteryValue` (`KismetMathLibrary.FMin` (+ _batteryvalue (* (`self.BatteryGeneratorChargeRate`) (`self.EngineUpdateSpeed`))) 100.0)))
  (message `/Game/BigRig/Widgets/BPI_RigWidget.UpdateBatteryGauge` (`WidgetComponent.GetWidget` (`self.BatteryWidget`)) (/ _output_get_2 100.0))
  (`/Game/BigRig/BPC_Interactable_ResourceDrain_Damagable.AddWear` (`self.BPC_Interactable_ResourceDrain_Damagable_Generator`) (`self.EngineUpdateSpeed`))
  (if (<= (`self.Fuel`) 0.0)
    (`self.Stop Engine`)
    (`self.StopGenerator`)))

(event `ReenableLights`
  ;[1 1 1] Lights
  (for _array_element (`self.LightArray`)
    (`SceneComponent.SetHiddenInGame` _array_element (not (`/Game/BigRig/BPC_DrainableLight.Active` _array_element)) true)))

(event `DisableLights`
  ;[1 1 1] Lights
  (for _array_element (`self.LightArray`)
    (`SceneComponent.SetHiddenInGame` _array_element true true)))

(event `self.BPC_Interactable_Switch_Engine.OnInteract`
  ;[1 1 1] Switches
  (if (`/Game/BigRig/BPC_Interactable_Switch.Value` (`self.BPC_Interactable_Switch_Engine`))
    (if (`/Game/BigRig/BPC_Interactable_ResourceDrain_Damagable.Damaged` (`self.BPC_Interactable_ResourceDrain_Damagable_Engine`))
      (`KismetSystemLibrary.PrintString` "Engine damaged")
      (set `/Game/BigRig/BPC_Interactable_Switch.Value` false (`self.BPC_Interactable_Switch_Engine`))
      (else
        (`self.Start Engine`)))
    (else
      (`self.Stop Engine`))))

(event `self.BPC_Interactable_ResourceDrain_Damagable_Engine.OnDamage`
  ;[1 1 1] Damage
  (`self.Stop Engine`))

(event `self.BPC_Interactable_ResourceDrain_Fuel.OnInteract`
  ;[1 1 1] Refueling
  (`self.Refuel` 30.0))

(event `self.BPC_Interactable_ResourceDrain_Damagable_Generator.OnDamage`
  ;[1 1 1] Damage
  (`self.StopGenerator`))

(event `Refuel`
  (params (Amount :type "Float (double-precision)"))
  ;[1 1 1] Refueling
  (bind _output_get (set `self.Fuel` (`KismetMathLibrary.FMin` (+ Amount (`self.Fuel`)) (`self.MaxFuel`))))
  (message `/Game/BigRig/Widgets/BPI_RigWidget.UpdateFuelGauge` (`WidgetComponent.GetWidget` (`self.FuelWidget`)) (/ _output_get (`self.MaxFuel`))))

(event `self.BPC_Interactable_ResourceDrain_Damagable_Battery.OnDamage`
  ;[1 1 1] Damage
  (`self.StopBattery`))

(event `self.BPC_Interactable_Switch_Generator.OnInteract`
  ;[1 1 1] Switches
  (if (`/Game/BigRig/BPC_Interactable_Switch.Value` (`self.BPC_Interactable_Switch_Generator`))
    (if (`/Game/BigRig/BPC_Interactable_ResourceDrain_Damagable.Damaged` (`self.BPC_Interactable_ResourceDrain_Damagable_Generator`))
      (`KismetSystemLibrary.PrintString` "Generator damaged")
      (set `/Game/BigRig/BPC_Interactable_Switch.Value` false (`self.BPC_Interactable_Switch_Generator`))
      (else
        (`self.StartGenerator`)))
    (else
      (`self.StopGenerator`))))

(event `self.BPC_Interactable_Switch_Battery.OnInteract`
  ;[1 1 1] Switches
  (if (`/Game/BigRig/BPC_Interactable_Switch.Value` (`self.BPC_Interactable_Switch_Battery`))
    (if (`/Game/BigRig/BPC_Interactable_ResourceDrain_Damagable.Damaged` (`self.BPC_Interactable_ResourceDrain_Damagable_Battery`))
      (`KismetSystemLibrary.PrintString` "Battery damaged")
      (set `/Game/BigRig/BPC_Interactable_Switch.Value` false (`self.BPC_Interactable_Switch_Battery`))
      (else
        (`self.StartBattery`)))
    (else
      (`self.StopBattery`))))

(event `self.ControlRig.OnPreInitializeDelegate`
  (params (Component :type "ControlRigComponent Object Reference"))
  (`ControlRigComponent.AddMappedCompleteSkeletalMesh` Component (`self.SkeletalMesh`)))

(fn `UserConstructionScript`
  (set `self.Fuel` (`self.MaxFuel`)))