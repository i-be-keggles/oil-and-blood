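; Actor component that plays footstep sounds for the owner's skeletal mesh in BigRig.
; On BeginPlay it collects socket and bone names starting with "Foot" but not ending in "end", printing an error without a mesh.
; Each tick it line-traces vertically through every foot, with debug drawing enabled.
; A per-foot grounded flag limits the sound, Teleport_Committed, to the moment a trace starts hitting after a miss.
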(event `self.ReceiveBeginPlay`
  (bind _returnvalue (`Actor.GetComponentByClass` (`self.GetOwner`) "/Script/Engine.SkeletalMeshComponent"))
  (`/Engine/EditorBlueprintResources/StandardMacros.IsValid` _returnvalue
    (:`Is Valid`
      (bind _output_get (set `self.Mesh` _returnvalue))
      (for _array_element (`SceneComponent.GetAllSocketNames` _output_get)
        (bind _returnvalue_2 (`KismetStringLibrary.Conv_NameToString` _array_element))
        (if (and (`KismetStringLibrary.StartsWith` _returnvalue_2 "Foot") (not (`KismetStringLibrary.EndsWith` _returnvalue_2 "end")))
          (`KismetArrayLibrary.Array_Add` (`self.Bones`) _array_element)
          (`KismetArrayLibrary.Array_Add` (`self.FootStates`) true))))
    (:`Is Not Valid`
      (`KismetSystemLibrary.PrintString` (`KismetStringLibrary.Concat_StrStr` (`KismetStringLibrary.Concat_StrStr` "Error: No skeletal mesh attached to (" (`KismetSystemLibrary.GetDisplayName` (`self.GetOwner`))) ") for footstep sounds.")))))

(event `Tick`
  (bind _footstates (`self.FootStates`))
  (for (_array_element _array_index) (`self.Bones`)
    (bind _returnvalue_location (`KismetMathLibrary.BreakTransform` (`SceneComponent.GetSocketTransform` (`self.Mesh`) _array_element "RTS_World")))
    (bind (_outhit _returnvalue) (`KismetSystemLibrary.LineTraceSingle` :`Start` (+ _returnvalue_location (0.0 0.0 20.0)) :`End` (+ _returnvalue_location (`KismetMathLibrary.MakeVector` 0.0 0.0 (* (`self.TraceLength`) -1.0))) :`TraceChannel` "TraceTypeQuery1" :`DrawDebugType` "ForDuration"))
    (if _returnvalue
      (if (not (`|GetArrayItem` _footstates _array_index))
        (`KismetArrayLibrary.Array_Set` _footstates _array_index true)
        (`GameplayStatics.SpawnSoundAtLocation` "/Engine/VREditor/Sounds/UI/Teleport_Committed.Teleport_Committed" _returnvalue_location (struct) 0.5 1.0 0.0 null null))
      (else
        (`KismetArrayLibrary.Array_Set` _footstates _array_index)))))