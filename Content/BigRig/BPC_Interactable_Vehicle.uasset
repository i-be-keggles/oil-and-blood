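; Scene component that lets the player enter and exit its owning vehicle Pawn by switching possession.
; Interact disables BP_FirstPersonCharacter, attaches it to the component and possesses the vehicle, caching and restoring the vehicle's velocity across the switch.
; IA_Interact repossesses and detaches the character, waits one frame-time delay, then re-enables it with the velocity cached on entry and teleports it to the component's location and facing.
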(event `self.ReceiveBeginPlay`
  (bind _aspawn (cast `Pawn` (`self.GetOwner`))
    (:`then`
      (set `self.Owner` _aspawn))
    (:`CastFailed`
      (`KismetSystemLibrary.PrintString` "Error: Vehicle is not pawn."))))

(event `EnhancedInput|/Game/FirstPerson/Input/Actions/IA_Interact`
  (params (ActionValue :type Boolean) (ElapsedSeconds :type "Float (double-precision)") (TriggeredSeconds :type "Float (double-precision)") (InputAction :type "InputAction Object Reference" :default "/Game/FirstPerson/Input/Actions/IA_Interact.IA_Interact"))
  (bind _playerpawn (`self.PlayerPawn`))
  (:`Triggered`
    (if ActionValue
      (if (`self.IsPossessed`)
        (set `self.IsPossessed` false)
        (`Controller.Possess` (`GameplayStatics.GetPlayerController` 0) (`self.PlayerPawn`))
        (`Actor.K2_DetachFromActor` (`self.PlayerPawn`) "KeepWorld" "KeepWorld" "KeepWorld")
        (`KismetSystemLibrary.Delay` (`GameplayStatics.GetWorldDeltaSeconds`))
        (bind _asbp_first_person_character (cast `/Game/Player/BP_FirstPersonCharacter` _playerpawn))
        (`/Game/Player/BP_FirstPersonCharacter.Enable` _asbp_first_person_character)
        (set `MovementComponent.Velocity` (`self.Velocity`) (`Character.CharacterMovement` _asbp_first_person_character))
        (`Actor.K2_SetActorLocationAndRotation` _playerpawn (`self.K2_GetComponentLocation`) (`KismetMathLibrary.Conv_VectorToRotator` (`self.GetForwardVector`)) false true)))))

(event `/Game/Player/BPI_Interactable.Interact`
  (bind _owner (`self.Owner`))
  (if (not (`self.IsPossessed`))
    (bind _output_get (set `self.PlayerPawn` (`GameplayStatics.GetPlayerPawn` 0)))
    (bind _asbp_first_person_character (cast `/Game/Player/BP_FirstPersonCharacter` _output_get))
    (`/Game/Player/BP_FirstPersonCharacter.Disable` _asbp_first_person_character)
    (`Actor.K2_AttachToComponent` _output_get self "None" "KeepWorld" "KeepWorld" "KeepRelative" false)
    (bind _output_get_2 (set `self.Velocity` (`Actor.GetVelocity` (`self.Owner`))))
    (`Controller.Possess` (`GameplayStatics.GetPlayerController` 0) _owner)
    (set `MovementComponent.Velocity` _output_get_2 (`Pawn.GetMovementComponent` _owner))
    (set `self.IsPossessed` true)))