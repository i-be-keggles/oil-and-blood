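; A BigRig interactable component that breaks down from wear and is repaired by spending a resource.
; AddWear accumulates wear until it reaches a randomized threshold, then Damage flags it, attaches a Niagara effect and calls OnDamage.
; Interacting while damaged repairs it if CheckAndConsume succeeds, removing the effect, calling OnRepair and re-rolling the threshold without clearing WearLevel.
; Observe returns the repair prompt only while damaged.
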(event `Damage`
  (set `self.Damaged` true)
  (bind _returnvalue (`NiagaraFunctionLibrary.SpawnSystemAttached` "/Game/FX/NS_DamagedComponent.NS_DamagedComponent" self "None" (0.0 0.0 0.0) (`KismetMathLibrary.Conv_VectorToRotator` (`self.GetForwardVector`)) "KeepRelativeOffset"))
  (set `self.Particles` _returnvalue)
  (`self.OnDamage`)
  (`KismetSystemLibrary.PrintString` "Component damaged"))

(event `Repair`
  (set `self.Damaged` false)
  (`self.K2_DestroyComponent` (`self.Particles`))
  (`self.OnRepair`)
  (`self.ResetWear`))

(event `/Game/Player/BPI_Interactable.Interact`
  (if (`self.Damaged`)
    (bind _succeeded (`self.CheckAndConsume`))
    (if _succeeded
      (`self.Repair`))))

(event `self.ReceiveBeginPlay`
  (`self.ResetWear`))

(event `ResetWear`
  (set `self.WearThreshold` (+ (`self.WearThresholdMin`) (* (`KismetMathLibrary.RandomFloat`) (- (`self.WearThresholdMax`) (`self.WearThresholdMin`))))))

(event `AddWear`
  (params (Amount :type "Float (double-precision)"))
  (if (not (`self.Damaged`))
    (bind _output_get (set `self.WearLevel` (+ (`self.WearLevel`) Amount)))
    (if (>= _output_get (`self.WearThreshold`))
      (`self.Damage`))))

(fn `Observe`
  (returns (Prompt :type String))
  (return (select `bool` (`self.Damaged`) :`false` "Repair unneeded" :`true` (`self.PromptText`))))